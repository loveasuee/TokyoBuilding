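; BP_Ch turns a building or room view by playing Level Sequences while the mouse is dragged horizontally.
; Tick samples cursor X after short delays, playing or pausing the current player and calling ChangeWay when drag direction flips.
; Instead of reverse playback, it swaps between paired sequences at the mirrored frame (MinusTime minus current).
; It also creates the W_Image UI and stores building and room turn speeds in an SV save game.
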(event EventTick
  (params (DeltaSeconds :type Float%20%28single-precision%29))
  (Utilities|FlowControl|Delay 0.2)
  (if (Variables|Default|GetIsMouseClicking)
    (Variables|Default|SetOldPos (Variables|Default|GetClickPos))
    (bind _returnvalue (Class|WidgetLayoutLibrary|GetMousePositiononViewport))
    (Variables|Default|SetClickPos (.x _returnvalue))
    (if (Variables|Default|GetIsJustClick)
      (if (< (- (Variables|Default|GetOldPos) (Variables|Default|GetClickPos)) 0.1)
        (if (Variables|Default|GetIsReversing)
          (Variables|Default|SetIsReversing false)
          (CallFunction|ChangeWay :!label _label)
          (Utilities|FlowControl|Delay 0.1)
          (Default|ToggleBuilding (Variables|Default|GetWidget) (Variables|Default|GetIsReversing)))
        (Sequencer|Player|Play (Variables|Default|GetCurrentPlayer) :!class /Script/MovieScene.MovieSceneSequencePlayer :!label _label_2)
        (elif (> (- (Variables|Default|GetOldPos) (Variables|Default|GetClickPos)) 0.1)
          (if (Variables|Default|GetIsReversing)
            (goto _label_2)
            (else
              (Variables|Default|SetIsReversing true)
              (goto _label)))
          (else
            (Sequencer|Player|Pause (Variables|Default|GetCurrentPlayer) :!label _label_3))))
      (else
        (Variables|Default|SetIsJustClick true)
        (goto _label_3)))
    (else
      (goto _label_3))))

(event EventBeginPlay
  (bind _returnvalue (UserInterface|CreateWidget "/Game/System/W_Image.W_Image_C" 0 self))
  (bind _output_get (Variables|Default|SetWidget _returnvalue))
  (UserInterface|Viewport|AddtoViewport _returnvalue 0)
  (Input|SetInputModeGameandUI (Game|GetPlayerController 0) _output_get "DoNotLock" true)
  (Variables|/Script/Engine.PlayerController|SetbShowMouseCursor (Game|GetPlayerController 0) true)
  (CallFunction|InitializeSeqBuilding)
  (CallFunction|CastSaveGame))

(event Input|ActionEvents|InputActionToggleChangeSpeed
  (params (Key :type Key%20Structure :default "None"))
  (:Pressed
    (Default|ToggleDebugUI (Variables|Default|GetWidget))))

(fn ConstructionScript)

(fn PlaySeqBuilding
  (bind _seq_p (Variables|Default|GetSeq_P))
  (bind _sequenceplayer (Variables|/Script/LevelSequence.LevelSequenceActor|GetSequencePlayer _seq_p))
  (Variables|Default|SetCurrentPlayer _sequenceplayer)
  (Sequencer|Player|Play _sequenceplayer :!class /Script/MovieScene.MovieSceneSequencePlayer)
  (Sequencer|Player|Pause _sequenceplayer))

(fn PlaySeqRoom
  (params (P_Seq :type Level%20Sequence%20Object%20Reference) (R_Seq :type Level%20Sequence%20Object%20Reference))
  (bind _seq_p (Variables|Default|GetSeq_P))
  (bind _sequenceplayer (Variables|/Script/LevelSequence.LevelSequenceActor|GetSequencePlayer _seq_p))
  (Class|LevelSequenceActor|SetSequence _seq_p P_Seq)
  (Class|LevelSequenceActor|SetSequence (Variables|Default|GetSeq_R) R_Seq)
  (Variables|Default|SetCurrentPlayer _sequenceplayer)
  (Sequencer|Player|Play _sequenceplayer :!class /Script/MovieScene.MovieSceneSequencePlayer)
  (Components|Timeline|SetPlayRate _sequenceplayer (Variables|/Game/System/SV.SV_C|GetTurnSpeed_Build (Variables|Default|GetSV)))
  (Sequencer|Player|Pause _sequenceplayer))

(fn ChangeWay
  (Sequencer|Player|Pause (Variables|Default|GetCurrentPlayer))
  (if (Variables|Default|GetIsReversing)
    (Variables|Default|SetCurrentPlayer (Variables|/Script/LevelSequence.LevelSequenceActor|GetSequencePlayer (Variables|Default|GetSeq_P)))
    (Components|Timeline|SetPlaybackPosition (Variables|Default|GetCurrentPlayer) (Utilities|Struct|MakeMovieSceneSequencePlaybackParams (Utilities|Struct|MakeFrameTime (Utilities|Struct|MakeFrameNumber (- (Variables|Default|GetMinusTime) (.value (.frame (Sequencer|Player|GetCurrentTime (Variables|/Script/LevelSequence.LevelSequenceActor|GetSequencePlayer (Variables|Default|GetSeq_R))))))) 0.0) 0.0 "" "Frame" "Play" false))
    (else
      (Variables|Default|SetCurrentPlayer (Variables|/Script/LevelSequence.LevelSequenceActor|GetSequencePlayer (Variables|Default|GetSeq_R)))
      (Components|Timeline|SetPlaybackPosition (Variables|Default|GetCurrentPlayer) (Utilities|Struct|MakeMovieSceneSequencePlaybackParams (Utilities|Struct|MakeFrameTime (Utilities|Struct|MakeFrameNumber (- (Variables|Default|GetMinusTime) (.value (.frame (Sequencer|Player|GetCurrentTime (Variables|/Script/LevelSequence.LevelSequenceActor|GetSequencePlayer (Variables|Default|GetSeq_P))))))) 0.0) 0.0 "" "Frame" "Play" false)))))

(fn InitializeSeqBuilding
  (bind _outactor (Sequencer|Player|CreateLevelSequencePlayer "/Game/Cinematics/Sequences/Sequence/S_Building.S_Building"))
  (Variables|Default|SetSeq_P _outactor)
  (Variables|Default|SetCurrentPlayer (Variables|/Script/LevelSequence.LevelSequenceActor|GetSequencePlayer _outactor))
  (bind _outactor_2 (Sequencer|Player|CreateLevelSequencePlayer "/Game/Cinematics/Sequences/Sequence/S_Building_R.S_Building_R"))
  (Variables|Default|SetSeq_R _outactor_2)
  (Sequencer|Player|Play (Variables|/Script/LevelSequence.LevelSequenceActor|GetSequencePlayer _outactor) :!class /Script/MovieScene.MovieSceneSequencePlayer)
  (Components|Timeline|SetPlayRate (Variables|/Script/LevelSequence.LevelSequenceActor|GetSequencePlayer _outactor_2) 4.5)
  (Sequencer|Player|Pause (Variables|/Script/LevelSequence.LevelSequenceActor|GetSequencePlayer _outactor)))

(fn InitializeSeqRoom
  (bind _outactor (Sequencer|Player|CreateLevelSequencePlayer "/Game/Cinematics/Sequences/Sequence/S_A1.S_A1"))
  (Variables|Default|SetSeq_P _outactor)
  (Variables|Default|SetCurrentPlayer (Variables|/Script/LevelSequence.LevelSequenceActor|GetSequencePlayer _outactor))
  (bind _outactor_2 (Sequencer|Player|CreateLevelSequencePlayer "/Game/Cinematics/Sequences/Sequence/S_RA1.S_RA1"))
  (Variables|Default|SetSeq_R _outactor_2)
  (Sequencer|Player|Play (Variables|/Script/LevelSequence.LevelSequenceActor|GetSequencePlayer _outactor) :!class /Script/MovieScene.MovieSceneSequencePlayer)
  (Components|Timeline|SetPlayRate (Variables|/Script/LevelSequence.LevelSequenceActor|GetSequencePlayer _outactor) (Variables|/Game/System/SV.SV_C|GetTurnSpeed_Room (Variables|Default|GetSV)))
  (Sequencer|Player|Pause (Variables|/Script/LevelSequence.LevelSequenceActor|GetSequencePlayer _outactor)))

(fn CastSaveGame
  (bind _returnvalue (SaveGame|DoesSaveGameExist (Variables|Default|GetSaveGameStr)))
  (if _returnvalue
    (bind _returnvalue_2 (SaveGame|LoadGamefromSlot (Variables|Default|GetSaveGameStr)))
    (bind _assv (Utilities|Casting|CastToSV _returnvalue_2))
    (Variables|Default|SetSV _assv)
    (else
      (bind _returnvalue_3 (SaveGame|CreateSaveGameObject "/Game/System/SV.SV_C"))
      (Variables|Default|SetSV _returnvalue_3)
      (SaveGame|SaveGametoSlot _returnvalue_3 (Variables|Default|GetSaveGameStr)))))

(fn UISetTurnSpeedBuild
  (params (Speed :type Float%20%28double-precision%29))
  (bind _sv (Variables|Default|GetSV))
  (Variables|/Game/System/SV.SV_C|SetTurnSpeed_Build _sv Speed)
  (SaveGame|SaveGametoSlot _sv (Variables|Default|GetSaveGameStr)))

(fn UISetTurnSpeedRoom
  (params (Speed :type Float%20%28double-precision%29))
  (bind _sv (Variables|Default|GetSV))
  (Variables|/Game/System/SV.SV_C|SetTurnSpeed_Room _sv Speed)
  (SaveGame|SaveGametoSlot _sv (Variables|Default|GetSaveGameStr)))